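; BP_Tunnel is a tunnel segment in an endless runner, with a rotating holed wall and optional enemy and health pack.
; Passing its trigger or surviving a wall hit destroys it and has TunnelSpawner spawn another; passing also raises the player's score and updates speed.
; Wall and enemy hits cost health and can trigger restart, packs heal, and bullets remove enemies for score or destroy packs.
; Helper functions randomize wall mesh, rotation, spin speed and pickup/enemy presence and placement.
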(event OnComponentBeginOverlap(HealthPack)
  (params (OverlappedComponent :type Primitive%20Component%20Object%20Reference) (OtherActor :type Actor%20Object%20Reference) (OtherComp :type Primitive%20Component%20Object%20Reference) (OtherBodyIndex :type Integer) (bFromSweep :type Boolean) (SweepResult :type Hit%20Result%20Structure%20%28by%20ref%29))
  (bind _asbp_player (Utilities|Casting|CastToBP_Player OtherActor)
    (:then
      (if (<= (+ (Variables|/Game/InfiniteMatrix/Blueprints/BP_Player.BP_Player_C|GetHealth _asbp_player) 20) 100)
        (Variables|/Game/InfiniteMatrix/Blueprints/BP_Player.BP_Player_C|SetHealth _asbp_player (+ (Variables|/Game/InfiniteMatrix/Blueprints/BP_Player.BP_Player_C|GetHealth _asbp_player) 20))
        (Default|UpdateHealth _asbp_player)
        (Components|DestroyComponent (Variables|Default|GetHealthPack))
        (else
          (Variables|/Game/InfiniteMatrix/Blueprints/BP_Player.BP_Player_C|SetHealth _asbp_player 100))))
    (:CastFailed
      (bind _asbp_bullet (Utilities|Casting|CastToBP_Bullet OtherActor))
      (Components|DestroyComponent (Variables|Default|GetHealthPack))
      (Actor|DestroyActor _asbp_bullet))))

(event OnComponentHit(WallMesh)
  (params (HitComponent :type Primitive%20Component%20Object%20Reference) (OtherActor :type Actor%20Object%20Reference) (OtherComp :type Primitive%20Component%20Object%20Reference) (NormalImpulse :type Vector :default "0, 0, 0") (Hit :type Hit%20Result%20Structure%20%28by%20ref%29))
  (bind _asbp_player (Utilities|Casting|CastToBP_Player OtherActor))
  (Variables|/Game/InfiniteMatrix/Blueprints/BP_Player.BP_Player_C|SetHealth _asbp_player (- (Variables|/Game/InfiniteMatrix/Blueprints/BP_Player.BP_Player_C|GetHealth _asbp_player) 20))
  (Default|UpdateHealth _asbp_player)
  (if (<= (Variables|/Game/InfiniteMatrix/Blueprints/BP_Player.BP_Player_C|GetHealth _asbp_player) 0)
    (Variables|/Game/InfiniteMatrix/Blueprints/BP_Player.BP_Player_C|SetIsDead _asbp_player true)
    (Default|DisplayRestart _asbp_player)
    (else
      (Actor|DestroyActor)
      (Default|SpawnTunnelatSpawnPoint (Variables|Default|GetTunnelSpawner)))))

(event OnComponentBeginOverlap(TriggerZone)
  (params (OverlappedComponent :type Primitive%20Component%20Object%20Reference) (OtherActor :type Actor%20Object%20Reference) (OtherComp :type Primitive%20Component%20Object%20Reference) (OtherBodyIndex :type Integer) (bFromSweep :type Boolean) (SweepResult :type Hit%20Result%20Structure%20%28by%20ref%29))
  (bind _asbp_player (Utilities|Casting|CastToBP_Player OtherActor))
  (Default|SpawnTunnelatSpawnPoint (Variables|Default|GetTunnelSpawner))
  (Actor|DestroyActor)
  (Utilities|FlowControl|Sequence
    (:then_0
      (Default|IncrementScore _asbp_player)
      (Default|UpdateSpeed _asbp_player))
    (:then_1
      (Default|UpdateScore _asbp_player))))

(event OnComponentBeginOverlap(Enemy)
  (params (OverlappedComponent :type Primitive%20Component%20Object%20Reference) (OtherActor :type Actor%20Object%20Reference) (OtherComp :type Primitive%20Component%20Object%20Reference) (OtherBodyIndex :type Integer) (bFromSweep :type Boolean) (SweepResult :type Hit%20Result%20Structure%20%28by%20ref%29))
  (bind _asbp_player (Utilities|Casting|CastToBP_Player OtherActor)
    (:then
      (Variables|/Game/InfiniteMatrix/Blueprints/BP_Player.BP_Player_C|SetHealth _asbp_player (- (Variables|/Game/InfiniteMatrix/Blueprints/BP_Player.BP_Player_C|GetHealth _asbp_player) 20))
      (Default|UpdateHealth _asbp_player)
      (if (<= (Variables|/Game/InfiniteMatrix/Blueprints/BP_Player.BP_Player_C|GetHealth _asbp_player) 0)
        (Variables|/Game/InfiniteMatrix/Blueprints/BP_Player.BP_Player_C|SetIsDead _asbp_player true)
        (Default|DisplayRestart _asbp_player)
        (else
          (Components|DestroyComponent (Variables|Default|GetEnemy)))))
    (:CastFailed
      (bind _asbp_bullet (Utilities|Casting|CastToBP_Bullet OtherActor))
      (Actor|DestroyActor _asbp_bullet)
      (bind _asbp_player_2 (Utilities|Casting|CastToBP_Player (Game|Player|GetPlayerPawn 0)))
      (Default|IncrementScore _asbp_player_2)
      (Default|UpdateScore _asbp_player_2)
      (Components|DestroyComponent (Variables|Default|GetEnemy)))))

(event EventBeginPlay)

(event EventTick
  (params (DeltaSeconds :type Float%20%28single-precision%29))
  (Transformation|AddLocalRotation (Variables|Default|GetWallMesh) (Math|Rotator|MakeRotator (* DeltaSeconds (Variables|Default|GetRotateSpeed)) 0.0 0.0) false false))

(fn ConstructionScript)

(fn RandomizeWall
  (Components|StaticMesh|SetStaticMesh (Variables|Default|GetWallMesh) (Utilities|Select :Index (Math|Random|RandomIntegerinRange 0 3) :Option%200 "/Game/InfiniteMatrix/Meshes/SM_Hole_01.SM_Hole_01" :Option%201 "/Game/InfiniteMatrix/Meshes/SM_Hole_02.SM_Hole_02" :Option%202 "/Game/InfiniteMatrix/Meshes/SM_Hole_03.SM_Hole_03" :Option%203 "/Game/InfiniteMatrix/Meshes/SM_Hole_04.SM_Hole_04"))
  (Transformation|AddLocalRotation (Variables|Default|GetWallMesh) (Math|Rotator|MakeRotator (Math|Random|RandomFloatinRange 0.0 3.6e+02) 0.0 0.0) false false))

(fn RandomRotate
  (Variables|Default|SetRotateSpeed (Math|Random|RandomFloatinRange -1e+02 1e+02)))

(fn SpawnEnemy
  (bind _enemy (Variables|Default|GetEnemy))
  (if (== (Math|Random|RandomIntegerinRange 0 2) 2)
    (Transformation|AddLocalOffset _enemy (Math|Vector|MakeVector 0.0 (Math|Random|RandomFloatinRange -2e+02 2e+02) (Math|Random|RandomFloatinRange -2e+02 2e+02)) false false)
    (else
      (Components|DestroyComponent _enemy))))

(fn SpawnHealthPack
  (bind _healthpack (Variables|Default|GetHealthPack))
  (if (== (Math|Random|RandomIntegerinRange 0 4) 4)
    (Transformation|AddLocalOffset _healthpack (Math|Vector|MakeVector (Math|Random|RandomFloatinRange -2e+02 2e+02) (Math|Random|RandomFloatinRange -4e+02 4e+02) (Math|Random|RandomFloatinRange -4e+02 4e+02)) false false)
    (else
      (Components|DestroyComponent _healthpack))))